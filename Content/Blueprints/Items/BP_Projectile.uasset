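; BP_Projectile is a projectile actor that deals damage to whatever its Collision component hits.
; On a hit, it stores the hit actor, impact point and surface normal.
; It spawns a Niagara spark effect at that point oriented along the normal, applies BaseDamage to the hit actor, then destroys itself.
; The construction script is empty.
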(event `self.Collision.OnComponentHit`
  (params (HitComponent :type "PrimitiveComponent Object Reference") (OtherActor :type "Actor Object Reference") (OtherComp :type "PrimitiveComponent Object Reference") (NormalImpulse :type "Vector Structure") (Hit :type "HitResult Structure (by ref)"))
  (set `self.Hit Actor` OtherActor)
  (set `self.Hit Impact Point` Hit_ImpactPoint)
  (set `self.Hit Impact Normal` Hit_ImpactNormal)
  (`|ExecutionSequence`
    (:`then_0`
      (`NiagaraFunctionLibrary.SpawnSystemAtLocation` "/Game/Effects/Particles/Impacts/NS_ImactSparksCharacter.NS_ImactSparksCharacter" (`self.Hit Impact Point`) (`KismetMathLibrary.Conv_VectorToRotator` (`self.Hit Impact Normal`))))
    (:`then_1`
      (`GameplayStatics.ApplyDamage` (`self.Hit Actor`) (`self.Base Damage`))
      (`self.K2_DestroyActor`))))

(fn `UserConstructionScript`)