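; BP_JumpItem is a pickup item that temporarily raises the player's jump velocity.
; On pickup it calls the parent logic, spawns a Niagara effect at the player, then hides its mesh and disables pickup collision.
; It caches the player's JumpZVelocity, adds the buff value, and runs a timeline that feeds its alpha into the player's JumpBuff.
; When the timeline finishes, it restores the cached velocity and destroys itself.
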(event `self.Pickup`
  (params (Player :type "/Game/Blueprints/Characters/Player/BP_Player Object Reference"))
  (bind _charactermovement (`Character.CharacterMovement` (`self.Player`)))
  (`parent.Pickup` Player)
  (`NiagaraFunctionLibrary.SpawnSystemAtLocation` "/Game/Effects/Particles/Item/NS_ItemPickup.NS_ItemPickup" (`self.K2_GetActorLocation` (`self.Player`)))
  (`SceneComponent.SetHiddenInGame` (`self.SkeletalMesh`) true false)
  (`PrimitiveComponent.SetCollisionEnabled` (`self.PickupArea`) "NoCollision")
  (bind _output_get (set `self.PrevJumpZVelocity` (`CharacterMovementComponent.JumpZVelocity` _charactermovement)))
  (set `CharacterMovementComponent.JumpZVelocity` (+ _output_get (`self.ZumpBuffValue`)) _charactermovement)
  (bind (_direction _alpha) (`Timeline|JumpItemTimeline`)
    (:`Update`
      (`/Game/Blueprints/Characters/Player/BP_Player.JumpBuff` (`self.Player`) _alpha))
    (:`Finished`
      (set `CharacterMovementComponent.JumpZVelocity` (`self.PrevJumpZVelocity`) _charactermovement)
      (`self.K2_DestroyActor`))))

(fn `UserConstructionScript`
  (`parent.UserConstructionScript`))