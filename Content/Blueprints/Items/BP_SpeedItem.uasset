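; BP_SpeedItem is a pickup that grants the player a temporary walk speed boost.
; On pickup it runs the parent logic, spawns a Niagara effect, hides its mesh, disables collision and adds SpeedBuffValue to MaxWalkSpeed.
; A timeline, named JumpItemTimeline, times the buff and feeds Alpha to the player's SpeedBuff.
; When it finishes, the item zeroes the player's buff value, subtracts the added speed and destroys itself.
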(event `self.Pickup`
  (params (Player :type "/Game/Blueprints/Characters/Player/BP_Player Object Reference"))
  (bind _player (`self.Player`))
  (bind _player_2 (`self.Player`))
  (bind _charactermovement (`Character.CharacterMovement` _player_2))
  (bind _charactermovement_2 (`Character.CharacterMovement` _player))
  (`parent.Pickup` Player)
  (`NiagaraFunctionLibrary.SpawnSystemAtLocation` "/Game/Effects/Particles/Item/NS_ItemPickup.NS_ItemPickup" (`self.K2_GetActorLocation` (`self.Player`)))
  (`SceneComponent.SetHiddenInGame` (`self.SkeletalMesh`) true false)
  (`PrimitiveComponent.SetCollisionEnabled` (`self.PickupArea`) "NoCollision")
  (bind _output_get (set `/Game/Blueprints/Characters/Player/BP_Player.SpeedBuffValue` (`self.SpeedBuffValue`) _player))
  (set `CharacterMovementComponent.MaxWalkSpeed` (+ _output_get (`CharacterMovementComponent.MaxWalkSpeed` _charactermovement_2)) _charactermovement_2)
  (bind (_direction _alpha) (`Timeline|JumpItemTimeline`)
    (:`Update`
      (`/Game/Blueprints/Characters/Player/BP_Player.SpeedBuff` _player_2 _alpha))
    (:`Finished`
      (set `/Game/Blueprints/Characters/Player/BP_Player.SpeedBuffValue` 0.0 _player_2)
      (set `CharacterMovementComponent.MaxWalkSpeed` (- (`CharacterMovementComponent.MaxWalkSpeed` _charactermovement) (`self.SpeedBuffValue`)) _charactermovement)
      (`self.K2_DestroyActor`))))

(fn `UserConstructionScript`
  (`parent.UserConstructionScript`))