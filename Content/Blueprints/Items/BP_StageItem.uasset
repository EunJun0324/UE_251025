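; BP_StageItem is a pickup item that sends the game to the next stage when collected.
; Tick spins its skeletal mesh in roll and yaw at RotateSpeed, holding pitch at zero.
; Pickup runs the parent logic, spawns the NS_StageChange Niagara effect and hides the mesh, then opens the NextStage level by name after a short delay.
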(event `self.ReceiveTick`
  (params (DeltaSeconds :type "Float (single-precision)"))
  (bind _skeletalmesh (`self.SkeletalMesh`))
  (bind _returnvalue (* DeltaSeconds (`self.RotateSpeed`)))
  (bind (_relativerotation_roll _relativerotation_pitch _relativerotation_yaw) (`KismetMathLibrary.BreakRotator` (`SceneComponent.RelativeRotation` _skeletalmesh)))
  (`SceneComponent.K2_SetRelativeRotation` _skeletalmesh (`KismetMathLibrary.MakeRotator` (+ _returnvalue _relativerotation_roll) 0.0 (+ _returnvalue _relativerotation_yaw)) false false))

(event `self.Pickup`
  (params (Player :type "/Game/Blueprints/Characters/Player/BP_Player Object Reference"))
  (`parent.Pickup` Player)
  (`NiagaraFunctionLibrary.SpawnSystemAtLocation` "/Game/Effects/Particles/Item/NS_StageChange.NS_StageChange" (`self.K2_GetActorLocation`))
  (`SceneComponent.SetHiddenInGame` (`self.SkeletalMesh`) true false)
  (`KismetSystemLibrary.Delay` 3.0)
  (`GameplayStatics.OpenLevel` (`self.NextStage`)))

(fn `UserConstructionScript`
  (`parent.UserConstructionScript`))