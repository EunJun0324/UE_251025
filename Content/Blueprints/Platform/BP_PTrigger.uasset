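; BP_PTrigger is a trigger that activates and deactivates an InteractionPlatform based on the actors inside its collision volume.
; Overlapping actors tagged "Interaction" are tracked in an array.
; The first arrival calls Interaction on the platform, and the last departure calls SecondInteraction.
; Unconnected nodes sum actor mass through BP_IMass, but mass does not affect triggering.
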(event `self.TriggerCollision.OnComponentBeginOverlap`
  (params (OverlappedComponent :type "PrimitiveComponent Object Reference") (OtherActor :type "Actor Object Reference") (OtherComp :type "PrimitiveComponent Object Reference") (OtherBodyIndex :type Integer) (bFromSweep :type Boolean) (SweepResult :type "HitResult Structure (by ref)"))
  (if (`self.ActorHasTag` OtherActor "Interaction")
    (`KismetArrayLibrary.Array_AddUnique` (`self.Interactions`) OtherActor)
    (if (== (`KismetArrayLibrary.Array_Length` (`self.Interactions`)) 1)
      (`/Game/Blueprints/Platform/BP_PInteraction.Interaction` (`self.InteractionPlatform`)))))

(event `self.TriggerCollision.OnComponentEndOverlap`
  (params (OverlappedComponent :type "PrimitiveComponent Object Reference") (OtherActor :type "Actor Object Reference") (OtherComp :type "PrimitiveComponent Object Reference") (OtherBodyIndex :type Integer))
  (if (`self.ActorHasTag` OtherActor "Interaction")
    (`KismetArrayLibrary.Array_RemoveItem` (`self.Interactions`) OtherActor)
    (if (== (`KismetArrayLibrary.Array_Length` (`self.Interactions`)) 0)
      (`/Game/Blueprints/Platform/BP_PInteraction.SecondInteraction` (`self.InteractionPlatform`)))))

(fn `UserConstructionScript`)