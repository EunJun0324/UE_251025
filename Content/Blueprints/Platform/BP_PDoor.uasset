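; BP_PDoor is a door that slides between its placed location and an offset position in response to interactions.
; On BeginPlay it caches the start location and adds Offset to get the end location.
; Interaction plays the Move timeline, which lerps the actor between both points without sweeping, and SecondInteraction reverses it.
; Both interaction events call their parent implementation first.
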(event `self.ReceiveBeginPlay`
  (bind _output_get (set `self.StartLocation` (`self.K2_GetActorLocation`)))
  (set `self.EndLocation` (+ _output_get (`self.Offset`))))

(event `self.Interaction`
  (`parent.Interaction`)
  (bind (_direction _alpha) (`Timeline|Move` :!label _label)
    (:`Update`
      (`self.K2_SetActorLocation` (`KismetMathLibrary.VLerp` (`self.StartLocation`) (`self.EndLocation`) _alpha)))))

(event `self.SecondInteraction`
  (`parent.SecondInteraction`)
  (goto _label :!via `Reverse`))

(fn `UserConstructionScript`
  (`parent.UserConstructionScript`))