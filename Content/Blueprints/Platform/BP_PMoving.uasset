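; BP_PMoving is a platform that shuttles back and forth between its starting point and an end point marked by EndMesh.
; On BeginPlay it stores both locations and destroys the marker mesh.
; Tick moves it by Speed per frame without delta-time scaling, flipping the target on arrival.
; A 1.5-second timer flag blocks repeated flips without pausing movement, and Tick prints that flag for debugging.
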(event `self.ReceiveBeginPlay`
  ;[0.15 0 0 0.5] BeginPlay
  (set `self.StartLocation` (`self.K2_GetActorLocation`))
  (set `self.EndLocation` (`SceneComponent.K2_GetComponentLocation` (`self.EndMesh`)))
  (`ActorComponent.K2_DestroyComponent` (`self.EndMesh`))
  (set `self.TargetLocation` (`self.EndLocation`))
  (set `self.bEnd` true))

(event `self.ReceiveTick`
  (params (DeltaSeconds :type "Float (single-precision)"))
  (`KismetSystemLibrary.PrintString` (`KismetStringLibrary.Conv_BoolToString` (`self.bEndTimer`)))
  (`self.K2_SetActorLocation` (+ (`self.K2_GetActorLocation`) (* (`KismetMathLibrary.Normal` (- (`self.TargetLocation`) (`self.K2_GetActorLocation`))) (`self.Speed`))))
  (if (and (`KismetMathLibrary.Vector_IsNearlyZero` (- (`self.K2_GetActorLocation`) (`self.TargetLocation`)) 5.0) (not (`self.bEndTimer`)))
    (set `self.bEndTimer` true)
    (`KismetSystemLibrary.K2_SetTimer` null "SetEndTimer" 1.5)
    (if (`self.bEnd`)
      (set `self.TargetLocation` (`self.StartLocation`))
      (set `self.bEnd` false)
      (else
        (set `self.TargetLocation` (`self.EndLocation`))
        (set `self.bEnd` true)))))

(event `SetEndTimer`
  (set `self.bEndTimer` false)
  (`KismetSystemLibrary.K2_ClearTimer` null "SetEndTimer"))

(fn `UserConstructionScript`
  (`parent.UserConstructionScript`))