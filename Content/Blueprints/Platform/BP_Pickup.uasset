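; BP_Pickup is a physics object that the player can pick up and drop.
; Overlapping its pickup area registers or clears it on BP_Player and toggles the prompt text in its WBP_PickupMessage widget.
; Pickup disables the cube's physics and attaches to the player mesh's Pickup socket, while UnPickup re-enables physics and detaches in place.
; GetMass exposes the cube's mass.
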(event `self.PickupArea.OnComponentBeginOverlap`
  (params (OverlappedComponent :type "PrimitiveComponent Object Reference") (OtherActor :type "Actor Object Reference") (OtherComp :type "PrimitiveComponent Object Reference") (OtherBodyIndex :type Integer) (bFromSweep :type Boolean) (SweepResult :type "HitResult Structure (by ref)"))
  (bind _asbp_player (cast `/Game/Blueprints/Characters/Player/BP_Player` OtherActor))
  (`/Game/Blueprints/Characters/Player/BP_Player.AddPickup` _asbp_player self)
  (bind _aswbp_pickup_message (cast `/Game/Blueprints/Widgets/WBP_PickupMessage` (`WidgetComponent.GetWidget` (`self.Widget`))))
  (`/Game/Blueprints/Widgets/WBP_PickupMessage.ShowTextPickup` _aswbp_pickup_message true))

(event `self.PickupArea.OnComponentEndOverlap`
  (params (OverlappedComponent :type "PrimitiveComponent Object Reference") (OtherActor :type "Actor Object Reference") (OtherComp :type "PrimitiveComponent Object Reference") (OtherBodyIndex :type Integer))
  (bind _asbp_player (cast `/Game/Blueprints/Characters/Player/BP_Player` OtherActor))
  (`/Game/Blueprints/Characters/Player/BP_Player.RemovePickup` _asbp_player)
  (bind _aswbp_pickup_message (cast `/Game/Blueprints/Widgets/WBP_PickupMessage` (`WidgetComponent.GetWidget` (`self.Widget`))))
  (`/Game/Blueprints/Widgets/WBP_PickupMessage.ShowTextPickup` _aswbp_pickup_message false))

(event `Pickup`
  (params (Player :type "/Game/Blueprints/Characters/Player/BP_Player Object Reference"))
  (`PrimitiveComponent.SetSimulatePhysics` (`self.Cube`) false)
  (`self.K2_AttachToComponent` (`Character.Mesh` Player) "Pickup" "SnapToTarget" "KeepRelative" "KeepRelative"))

(event `UnPickup`
  (`PrimitiveComponent.SetSimulatePhysics` (`self.Cube`) true)
  (`self.K2_DetachFromActor` "KeepWorld"))

(fn `GetMass`
  (returns (Mass :type "Float (double-precision)"))
  (return (`PrimitiveComponent.GetMass` (`self.Cube`))))

(fn `UserConstructionScript`)