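; Enemy AI controller that turns its pawn toward a sensed actor and then moves to it.
; On a successful perception update, it captures the current rotation and the look-at rotation to the target.
; A timeline lerps the pawn between them, and MoveToActor starts once the timeline finishes.
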(event `self.AIPerception.OnTargetPerceptionUpdated`
  (params (Actor :type "Actor Object Reference") (Stimulus :type "AIStimulus Structure"))
  (bind _returnvalue (`self.K2_GetPawn`))
  (if Stimulus_bSuccessfullySensed
    (set `self.StartRotation` (`self.K2_GetActorRotation` _returnvalue))
    (set `self.TargetRotation` (`KismetMathLibrary.FindLookAtRotation` (`self.K2_GetActorLocation` _returnvalue) (`self.K2_GetActorLocation` Actor)))
    (bind (_direction _alpha) (`Timeline|타임라인` :!via `PlayFromStart`)
      (:`Update`
        (`self.K2_SetActorRotation` (`self.K2_GetPawn`) (`KismetMathLibrary.RLerp` (`self.StartRotation`) (`self.TargetRotation`) _alpha) false))
      (:`Finished`
        (`self.MoveToActor` Actor -1.0 true true true null)))))

(fn `UserConstructionScript`)