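; BP_Enemy is a damageable enemy with hit points that flashes when hit and dies when they run out.
; On BeginPlay it fills its health, swaps each mesh material for a stored dynamic instance and hides its EndPoint component in game.
; Non-lethal damage plays a timeline that drives the "Red" parameter on those materials.
; Lethal damage marks it dead, turns on mesh physics and sets a short lifespan before removal.
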(event `self.ReceiveBeginPlay`
  (set `self.Hp` (`self.MaxHp`))
  (for (_array_element _array_index) (`MeshComponent.GetMaterials` (`self.Mesh`))
    (bind _returnvalue (`KismetMaterialLibrary.CreateDynamicMaterialInstance` _array_element))
    (`KismetArrayLibrary.Array_Add` (`self.MaterialDynamics`) _returnvalue)
    (`PrimitiveComponent.SetMaterial` (`self.Mesh`) _array_index _returnvalue))
  (`SceneComponent.SetHiddenInGame` (`self.EndPoint`) true false))

(event `self.ReceiveAnyDamage`
  (params (Damage :type "Float (single-precision)") (DamageType :type "DamageType Object Reference") (InstigatedBy :type "Controller Object Reference") (DamageCauser :type "Actor Object Reference"))
  (if (not (`self.bDied`))
    (bind _output_get (set `self.Hp` (- (`self.Hp`) Damage)))
    (if (<= _output_get 0.0)
      (set `self.bDied` true)
      (`PrimitiveComponent.SetSimulatePhysics` (`self.Mesh`) true)
      (`self.SetLifeSpan` 4.0)
      (else
        (bind (_direction _redvalue) (`Timeline|HitTimeline` :!via `PlayFromStart`)
          (:`Update`
            (for _array_element (`self.MaterialDynamics`)
              (`MaterialInstanceDynamic.SetVectorParameterValue` _array_element "Red" (make `LinearColor` _redvalue)))))))))

(fn `UserConstructionScript`)