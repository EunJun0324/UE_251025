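; Third-person player character that moves, runs, jumps, aims, fires an equipped weapon and carries one pickup at a time.
; Enhanced Input drives actions: aiming shortens the spring arm and animates FOV through a timeline, while auto-fire repeats shots on a looping timer.
; External calls attach weapons to a hand socket and register nearby pickups.
; A HUD widget created on BeginPlay shows crosshair, auto-fire state and jump/speed buff progress.
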(event `self.ReceiveBeginPlay`
  ;[0.15 0 0 0.5] BeginPlay
  (`|ExecutionSequence`
    (:`then_0`
      (bind `_as플레이어_컨트롤러` (cast `PlayerController` (`self.GetController`)))
      (`EnhancedInputSubsystemInterface.AddMappingContext` (pcsubsystem `EnhancedInputLocalPlayerSubsystem` `_as플레이어_컨트롤러`) "/Game/Blueprints/Input/IMC_Player.IMC_Player" 0 (struct)))
    (:`then_1`
      (bind _returnvalue (`|CreateWidget` "/Game/Blueprints/Widgets/WBP_PlayerHUD.WBP_PlayerHUD_C" (`GameplayStatics.GetPlayerController` 0)))
      (bind _output_get (set `self.PlayerWidget` _returnvalue))
      (`UserWidget.AddToViewport` _output_get 0)
      (`/Game/Blueprints/Widgets/WBP_PlayerHUD.ShowCrosshair` (`self.PlayerWidget`) false)
      (`/Game/Blueprints/Widgets/WBP_PlayerHUD.ToggleAutoFire` (`self.PlayerWidget`) (`self.AutoFire`)))))

(event `Equip`
  (params (Weapon :type "/Game/Blueprints/Items/BP_Weapon Object Reference"))
  ;[0.15 0 0 0.5] Equip
  (`self.SetOwner` Weapon self)
  (`self.K2_AttachToComponent` Weapon (`self.Mesh`) "weapon_r" "SnapToTarget" "KeepRelative" "KeepRelative" true)
  (set `self.Equipped` true)
  (set `self.EquippedWeapon` Weapon))

(event `EnhancedInput|/Game/Blueprints/Input/IA_Move`
  (params (ActionValue :type "Vector2D Structure") (ElapsedSeconds :type "Float (double-precision)") (TriggeredSeconds :type "Float (double-precision)") (InputAction :type "InputAction Object Reference" :default "/Game/Blueprints/Input/IA_Move.IA_Move"))
  (bind (_returnvalue_roll _returnvalue_pitch _returnvalue_yaw) (`KismetMathLibrary.BreakRotator` (`self.GetControlRotation`)))
  (bind _returnvalue (`KismetMathLibrary.MakeRotator` 0.0 0.0 _returnvalue_yaw))
  (:`Triggered`
    (`self.AddMovementInput` (`KismetMathLibrary.GetForwardVector` _returnvalue) ActionValue_X)
    (`self.AddMovementInput` (`KismetMathLibrary.GetRightVector` _returnvalue) ActionValue_Y)))

(event `EnhancedInput|/Game/Blueprints/Input/IA_Look`
  (params (ActionValue :type "Vector2D Structure") (ElapsedSeconds :type "Float (double-precision)") (TriggeredSeconds :type "Float (double-precision)") (InputAction :type "InputAction Object Reference" :default "/Game/Blueprints/Input/IA_Look.IA_Look"))
  (:`Triggered`
    (`self.AddControllerYawInput` ActionValue_X)
    (`self.AddControllerPitchInput` (* ActionValue_Y -1.0))))

(event `EnhancedInput|/Game/Blueprints/Input/IA_Run`
  (params (ActionValue :type Boolean) (ElapsedSeconds :type "Float (double-precision)") (TriggeredSeconds :type "Float (double-precision)") (InputAction :type "InputAction Object Reference" :default "/Game/Blueprints/Input/IA_Run.IA_Run"))
  (bind _charactermovement (`self.CharacterMovement`))
  (:`Started`
    (set `CharacterMovementComponent.MaxWalkSpeed` (+ (`self.RunSpeed`) (`self.SpeedBuffValue`)) _charactermovement))
  (:`Completed`
    (set `CharacterMovementComponent.MaxWalkSpeed` (+ (`self.WalkSpeed`) (`self.SpeedBuffValue`)) _charactermovement)))

(event `EnhancedInput|/Game/Blueprints/Input/IA_Jump`
  (params (ActionValue :type Boolean) (ElapsedSeconds :type "Float (double-precision)") (TriggeredSeconds :type "Float (double-precision)") (InputAction :type "InputAction Object Reference" :default "/Game/Blueprints/Input/IA_Jump.IA_Jump"))
  (:`Started`
    (`self.Jump`)))

(event `EnhancedInput|/Game/Blueprints/Input/IA_Aim`
  (params (ActionValue :type Boolean) (ElapsedSeconds :type "Float (double-precision)") (TriggeredSeconds :type "Float (double-precision)") (InputAction :type "InputAction Object Reference" :default "/Game/Blueprints/Input/IA_Aim.IA_Aim"))
  (bind _springarm (`self.SpringArm`))
  ;[0.15 0 0 0.5] Aim
  (:`Started`
    (if (`self.Equipped`) :!label _label
      (if (`self.Aimming`)
        (set `SpringArmComponent.TargetArmLength` 300.0 _springarm)
        (set `self.Aimming` false)
        (bind (_direction _fov) (`Timeline|Aim` :!via `ReverseFromEnd` :!label _label_2)
          (:`Update`
            (set `CameraComponent.FieldOfView` _fov (`self.Camera`)))
          (:`Finished`
            (`/Game/Blueprints/Widgets/WBP_PlayerHUD.ShowCrosshair` (`self.PlayerWidget`) (`self.Aimming`))))
        (else
          (set `SpringArmComponent.TargetArmLength` 100.0 _springarm)
          (set `self.Aimming` true)
          (goto _label_2 :!via `PlayFromStart`)))))
  (:`Completed`
    (goto _label)))

(event `ShootEvent`
  ;[0.15 0 0 0.5] Fire
  (`/Game/Blueprints/Items/BP_Weapon.Shoot` (`self.EquippedWeapon`))
  (`self.PlayAnimMontage` "/Game/Animations/Actions/Fire_Montage.Fire_Montage"))

(event `EnhancedInput|/Game/Blueprints/Input/IA_Fire`
  (params (ActionValue :type Boolean) (ElapsedSeconds :type "Float (double-precision)") (TriggeredSeconds :type "Float (double-precision)") (InputAction :type "InputAction Object Reference" :default "/Game/Blueprints/Input/IA_Fire.IA_Fire"))
  ;[0.15 0 0 0.5] Fire
  (:`Started`
    (`self.EquippedWeapon`
      (:`then`
        (`self.ShootEvent`)
        (if (`self.AutoFire`)
          (`KismetSystemLibrary.K2_SetTimer` null "ShootEvent" (`self.ShootInterval`) true)))
      (:`else`)))
  (:`Completed`
    (`KismetSystemLibrary.K2_ClearTimer` null "ShootEvent")))

(event `EnhancedInput|/Game/Blueprints/Input/IA_AutoFire`
  (params (ActionValue :type Boolean) (ElapsedSeconds :type "Float (double-precision)") (TriggeredSeconds :type "Float (double-precision)") (InputAction :type "InputAction Object Reference" :default "/Game/Blueprints/Input/IA_AutoFire.IA_AutoFire"))
  ;[0.15 0 0 0.5] AutoFire
  (:`Started`
    (bind _output_get (set `self.AutoFire` (not (`self.AutoFire`))))
    (`/Game/Blueprints/Widgets/WBP_PlayerHUD.ToggleAutoFire` (`self.PlayerWidget`) _output_get)
    (if (not (`self.AutoFire`))
      (`KismetSystemLibrary.K2_ClearTimer` null "ShootEvent"))))

(event `EnhancedInput|/Game/Blueprints/Input/IA_Pickup`
  (params (ActionValue :type Boolean) (ElapsedSeconds :type "Float (double-precision)") (TriggeredSeconds :type "Float (double-precision)") (InputAction :type "InputAction Object Reference" :default "/Game/Blueprints/Input/IA_Pickup.IA_Pickup"))
  (:`Started`
    (bind _pickup (`self.Pickup`)
      (:`then`
        (`/Game/Blueprints/Platform/BP_Pickup.UnPickup` _pickup)
        (set `self.Pickup` null))
      (:`else`
        (bind _nearpickup (`self.NearPickup`)
          (:`then`
            (bind _output_get (set `self.Pickup` _nearpickup))
            (`/Game/Blueprints/Platform/BP_Pickup.Pickup` _output_get self)
            (`self.RemovePickup`))
          (:`else`))))))

(event `AddPickup`
  (params (Item :type "/Game/Blueprints/Platform/BP_Pickup Object Reference"))
  (set `self.NearPickup` Item))

(event `RemovePickup`
  (set `self.NearPickup` null))

(event `JumpBuff`
  (params (InPercent :type "Float (single-precision)"))
  (`/Game/Blueprints/Widgets/WBP_PlayerHUD.SetJumpProgressbar` (`self.PlayerWidget`) InPercent))

(event `SpeedBuff`
  (params (InPercent :type "Float (single-precision)"))
  (`/Game/Blueprints/Widgets/WBP_PlayerHUD.SetSpeedProgressbar` (`self.PlayerWidget`) InPercent))

(fn `GetMass`
  (returns (Mass :type "Float (double-precision)"))
  (return (`PrimitiveComponent.GetMass` (`self.CapsuleComponent`))))

(fn `UserConstructionScript`)