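; BP_Player is the player character, handling movement, camera look, running, jumping and weapon firing through Enhanced Input.
; BeginPlay adds the IMC_Player mapping context, and movement follows the control rotation's yaw while run input switches the max walk speed.
; Equip snaps a passed-in weapon to the weapon_r mesh socket and stores it, and fire input calls Shoot on that weapon when valid.
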(event `self.ReceiveBeginPlay`
  (bind `_as플레이어_컨트롤러` (cast `PlayerController` (`self.GetController`)))
  (`EnhancedInputSubsystemInterface.AddMappingContext` (pcsubsystem `EnhancedInputLocalPlayerSubsystem` `_as플레이어_컨트롤러`) "/Game/Blueprints/Input/IMC_Player.IMC_Player" 0 (struct)))

(event `EnhancedInput|/Game/Blueprints/Input/IA_Move`
  (params (ActionValue :type "Vector2D Structure") (ElapsedSeconds :type "Float (double-precision)") (TriggeredSeconds :type "Float (double-precision)") (InputAction :type "InputAction Object Reference" :default "/Game/Blueprints/Input/IA_Move.IA_Move"))
  (bind (_returnvalue_roll _returnvalue_pitch _returnvalue_yaw) (`KismetMathLibrary.BreakRotator` (`self.GetControlRotation`)))
  (bind _returnvalue (`KismetMathLibrary.MakeRotator` 0.0 0.0 _returnvalue_yaw))
  (:`Triggered`
    (`self.AddMovementInput` (`KismetMathLibrary.GetForwardVector` _returnvalue) ActionValue_X)
    (`self.AddMovementInput` (`KismetMathLibrary.GetRightVector` _returnvalue) ActionValue_Y)))

(event `EnhancedInput|/Game/Blueprints/Input/IA_Look`
  (params (ActionValue :type "Vector2D Structure") (ElapsedSeconds :type "Float (double-precision)") (TriggeredSeconds :type "Float (double-precision)") (InputAction :type "InputAction Object Reference" :default "/Game/Blueprints/Input/IA_Look.IA_Look"))
  (:`Triggered`
    (`self.AddControllerYawInput` ActionValue_X)
    (`self.AddControllerPitchInput` (* ActionValue_Y -1.0))))

(event `EnhancedInput|/Game/Blueprints/Input/IA_Run`
  (params (ActionValue :type Boolean) (ElapsedSeconds :type "Float (double-precision)") (TriggeredSeconds :type "Float (double-precision)") (InputAction :type "InputAction Object Reference" :default "/Game/Blueprints/Input/IA_Run.IA_Run"))
  (bind _charactermovement (`self.CharacterMovement`))
  (:`Started`
    (set `CharacterMovementComponent.MaxWalkSpeed` 600.0 _charactermovement))
  (:`Completed`
    (set `CharacterMovementComponent.MaxWalkSpeed` 400.0 _charactermovement)))

(event `EnhancedInput|/Game/Blueprints/Input/IA_Jump`
  (params (ActionValue :type Boolean) (ElapsedSeconds :type "Float (double-precision)") (TriggeredSeconds :type "Float (double-precision)") (InputAction :type "InputAction Object Reference" :default "/Game/Blueprints/Input/IA_Jump.IA_Jump"))
  (:`Started`
    (`self.Jump`)))

(event `Equip`
  (params (Weapon :type "/Game/Blueprints/Items/BP_Weapon Object Reference"))
  (`self.K2_AttachToComponent` Weapon (`self.Mesh`) "weapon_r" "SnapToTarget" "KeepRelative" "KeepRelative" true)
  (set `self.Equipped` true)
  (set `self.EquippedWeapon` Weapon))

(event `EnhancedInput|/Game/Blueprints/Input/IA_Fire`
  (params (ActionValue :type Boolean) (ElapsedSeconds :type "Float (double-precision)") (TriggeredSeconds :type "Float (double-precision)") (InputAction :type "InputAction Object Reference" :default "/Game/Blueprints/Input/IA_Fire.IA_Fire"))
  (:`Started`
    (bind _equippedweapon (`self.EquippedWeapon`)
      (:`then`
        (`/Game/Blueprints/Items/BP_Weapon.Shoot` _equippedweapon))
      (:`else`))))

(fn `UserConstructionScript`)